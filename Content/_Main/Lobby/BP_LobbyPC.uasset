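; Lobby player controller that manages a player's lobby UI, character selection and settings in a multiplayer session.
; It saves player info to a slot and reports changes to the lobby game mode, which updates everyone.
; Update events push characters, player list, map info and player count into the lobby widget.
; It also shows the loading screen and destroys the session on kick or EndPlay; chat handling is empty.
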(event Custom|InitialSetup
  ;[1 1 1] Tells server to update
  (CallFunction|SaveGame)
  (CallFunction|CallUpdate (Variables|Default|GetPlayerSettings) false))

(event Custom|SetupLobbyMenu
  (params (ServerName :type Text))
  ;[1 1 1] Setup and display lobby to all players
  (Variables|Default|SetbShowMouseCursor true)
  (bind _returnvalue (UserInterface|CreateWidget "/Game/_Main/Lobby/LobbyMenu.LobbyMenu_C" 0 ServerName))
  (bind _output_get (Variables|Default|SetLobbyWidget _returnvalue))
  (UserInterface|Viewport|AddtoViewport _output_get 0)
  (Input|SetInputModeGameandUI self (Variables|Default|GetLobbyWidget) "DoNotLock" true))

(event Custom|AddPlayerInfo
  (params (ConnectedPlayersInfo :type Array%20of%20S%20Player%20Info%20Structures))
  ;[1 1 1] Update Plyer List Info
  (Variables|Default|SetAllConnectedPlayers ConnectedPlayersInfo)
  (bind _lobbywidget (Variables|Default|GetLobbyWidget)
    (:then
      (Default|ClearPlayerList _lobbywidget)
      (for _array_element (Variables|Default|GetAllConnectedPlayers)
        (Default|UpdatePlayerWIndow (Variables|Default|GetLobbyWidget))))
    (:else)))

(event Custom|UpdateAvailableCharacter
  (params (AvailableCharacters :type Array%20of%20Booleans))
  ;[1 1 1] Update Client which character sare available
  (Variables|Default|SetAvailableCharacters AvailableCharacters)
  (bind _lobbywidget (Variables|Default|GetLobbyWidget)
    (:then
      (Default|UpdateCharactersAvailable _lobbywidget (Variables|Default|GetAvailableCharacters)))
    (:else)))

(event Custom|AddPlayerToKickWindow
  ;[1 1 1] Add player to kick window
  (bind _lobbywidget (Variables|Default|GetLobbyWidget)
    (:then
      (Default|AddPlayertoKickWindow _lobbywidget))
    (:else)))

(event Custom|SaveGame
  ;[1 1 1] Saves The player info
  (Variables|Default|GetPlayerSaveGameRef
    (:then
      _)
    (:else
      (bind _returnvalue (SaveGame|CreateSaveGameObject "/Game/_Main/PlayerSave.PlayerSave_C"))
      (bind _output_get (Variables|Default|SetPlayerSaveGameRef _returnvalue))))
  (Variables|/Game/_Main/PlayerSave.PlayerSave_C|SetPlayerInfo _output_get (Variables|Default|GetPlayerSettings))
  (SaveGame|SaveGametoSlot _output_get (Variables|Default|GetPlayerSettingsSave)))

(event Custom|GetChatMessage
  (params (TextToSend :type Text)))

(event Custom|UpdateLobbySettings
  (params (MapImage :type Texture%202D%20Object%20Reference) (MapName :type Text) (MapTime :type Text))
  ;[1 1 1] Updates client Lobby Info
  (Default|UpdateLobbyInfo (Variables|Default|GetLobbyWidget) MapImage MapName MapTime))

(event Custom|CallUpdate
  (params (PlayerSettings :type S%20Player%20Info%20Structure) (ChangedStatus? :type Boolean))
  ;[1 1 1] Assigns the updated selected character and tells the server to update
  (bind _output_get (Variables|Default|SetPlayerSettings PlayerSettings))
  (bind _lobbygm (Class|BPILobbyGM|LobbyGMRef(Message) (Game|GetGameMode)))
  (Default|ChangeCharcter _lobbygm self (Utilities|Struct|BreakS_PlayerInfo _output_get) ChangedStatus?)
  (Default|EveryoneUpdate _lobbygm))

(event Custom|ShowLoadingScreen
  ;[1 1 1] Removes lobby widget and displays loading screen when level loads in background
  (Widget|RemovefromParent (Variables|Default|GetLobbyWidget))
  (bind _returnvalue (UserInterface|CreateWidget "/Game/_Main/Widgets/LoadingScreen.LoadingScreen_C" self))
  (UserInterface|Viewport|AddtoViewport _returnvalue 0))

(event Custom|Kicked
  ;[1 1 1] Called when the serve rdisconnects or someone is kicked
  (Game|OpenLevel(byName) "MainMenu")
  (|DestroySession self))

(event Custom|AssignSelectedCharacter
  (params (SelectedCharacter :type Integer) (CharacterImage :type Texture%202D%20Object%20Reference))
  ;[1 1 1] Handle character selection adn determine if selected character is available to be assined
  (Variables|Default|SetPreviousSelection (Variables|Default|GetSelectedCharacter))
  (Variables|Default|SetCharacterImage CharacterImage)
  (Variables|Default|SetSelectedCharacter SelectedCharacter)
  (CallFunction|CharacterCheck))

(event Custom|CharacterCheck
  ;[1 1 1] Checks if selected character is available andif so assigns it to player
  (bind _lobbygm (Class|BPILobbyGM|LobbyGMRef(Message) (Game|GetGameMode)))
  (if (Utilities|Array|Get(acopy) (Variables|/Game/_Main/Lobby/BP_LobbyGameMode.BP_LobbyGameMode_C|GetAvailableCharacters _lobbygm) (Variables|Default|GetSelectedCharacter))
    _
    (else
      (Utilities|Array|SetArrayElem (Variables|/Game/_Main/Lobby/BP_LobbyGameMode.BP_LobbyGameMode_C|GetAvailableCharacters _lobbygm) (Variables|Default|GetSelectedCharacter) true)))
  (Utilities|Array|SetArrayElem (Variables|/Game/_Main/Lobby/BP_LobbyGameMode.BP_LobbyGameMode_C|GetAvailableCharacters _lobbygm) (Variables|Default|GetPreviousSelection) false)
  (CallFunction|AssignPlayer (Variables|Default|GetCharacterImage) (Utilities|Array|Get(acopy) (Variables|/Game/_Main/Lobby/BP_LobbyGameMode.BP_LobbyGameMode_C|GetCharacters _lobbygm) (Variables|Default|GetSelectedCharacter))))

(event Custom|AssignPlayer
  (params (PlayerImage :type Texture%202D%20Object%20Reference) (PlayerCharacter :type Character%20Class%20Reference))
  (bind _playersettings (Variables|Default|GetPlayerSettings))
  ;[1 1 1] Assigns selected character and updates everyone
  (Utilities|Struct|SetmembersinS_PlayerInfo _playersettings PlayerImage PlayerCharacter)
  (CallFunction|SaveGame)
  (CallFunction|CallUpdate _playersettings false))

(event Custom|UpdateNumebrOfPlayers
  (params (CurrentPlayers :type Integer) (MaxPlayers :type Integer))
  ;[1 1 1] Update and display numbe rof players
  (Default|UpdatePlayersDisplay (Variables|Default|GetLobbyWidget) (Utilities|Text|FormatText "{CurrentPlayers} of {MaxPlayers}" (Utilities|Text|ToText(Integer) CurrentPlayers) (Utilities|Text|ToText(Integer) MaxPlayers))))

(event EventEndPlay
  (params (EndPlayReason :type EEndPlayReason%20Enum :default "Destroyed"))
  ;[1 1 1] Called when the serve rdisconnects or someone is kicked
  (|DestroySession self))

(fn ConstructionScript)

(fn LobbyPCRef
  (return self))