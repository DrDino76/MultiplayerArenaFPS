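; Multiplayer lobby game mode that tracks connected players, host map settings, character choices and kicks.
; Login and logout feed EveryoneUpdate, which pushes player info, counts and available characters to each lobby controller and sets CanWeStart; logout also frees the character.
; Character changes spawn and possess a pawn at the last PlayerStart found.
; Launch shows loading screens on every client, then server-travels to the map matching the selected ID.
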(event Custom|SpawnPlayer
  (params (Player :type Player%20Controller%20Object%20Reference)))

(event Custom|StartLoadingScreen
  ;[1 1 1] Show loading screen and loads level
  (for _array_element (Variables|Default|GetConnectedPlayers)
    (bind _lobbypc (Class|BPILobbyPC|LobbyPCRef(Message) _array_element))
    (Default|ShowLoadingScreen _lobbypc))
  (CallFunction|LaunchGame))

(event Custom|HostUpdateGameSettings
  (params (SelectedMapImagre :type Texture%202D%20Object%20Reference) (SelectedMapName :type Text) (SelectedMapTime :type Text) (SelectedMapID :type Integer))
  ;[1 1 1] cahnges made clients update
  (Variables|Default|SetSelectedMapImagre SelectedMapImagre)
  (Variables|Default|SetSelectedMapName SelectedMapName)
  (Variables|Default|SetSelectedMapTime SelectedMapTime)
  (Variables|Default|SetSelectedMapID SelectedMapID)
  (for _array_element (Variables|Default|GetConnectedPlayers)
    (bind _lobbypc (Class|BPILobbyPC|LobbyPCRef(Message) _array_element))
    (Default|UpdateLobbySettings _lobbypc (Variables|Default|GetSelectedMapImagre) (Variables|Default|GetSelectedMapName) (Variables|Default|GetSelectedMapTime))))

(event Custom|PlayerKicked
  (params (PlayerID :type Integer))
  ;[1 1 1] Kick Selected Player
  (bind _lobbypc (Class|BPILobbyPC|LobbyPCRef(Message) (Utilities|Array|Get(acopy) (Variables|Default|GetConnectedPlayers) PlayerID)))
  (Default|Kicked _lobbypc))

(event Custom|EveryoneUpdate
  (bind _connectedplayers (Variables|Default|GetConnectedPlayers))
  (bind _connectplayersinfo (Variables|Default|GetConnectPlayersInfo))
  ;[1 1 1] Updates All Connected players for lobby widget
  (bind _output_get (Variables|Default|SetCurrentPlayers (Utilities|Array|Length (Variables|Default|GetConnectedPlayers))))
  (if (> _output_get 0)
    (Utilities|Array|Clear (Variables|Default|GetConnectPlayersInfo))
    (for _array_element _connectedplayers
      (bind _lobbypc (Class|BPILobbyPC|LobbyPCRef(Message) _array_element))
      (Utilities|Array|AddUnique _connectplayersinfo (Variables|/Game/_Main/Lobby/BP_LobbyPC.BP_LobbyPC_C|GetPlayerSettings _lobbypc))
      (Default|UpdateNumebrOfPlayers _lobbypc (Variables|Default|GetCurrentPlayers) (Variables|Default|GetMaxPlayers)))
    (for _array_element_2 _connectedplayers
      (bind _lobbypc_2 (Class|BPILobbyPC|LobbyPCRef(Message) _array_element_2))
      (Default|AddPlayerInfo _lobbypc_2 _connectplayersinfo)
      (Default|UpdateAvailableCharacter _lobbypc_2 (Variables|Default|GetAvailableCharacters))
      (CallFunction|AddtoKickList))
    (bind _array_element_3 (Utilities|Array|ForEachLoopwithBreak (Variables|Default|GetConnectPlayersInfo))
      (:LoopBody
        (if (== (.PlayerCharacter (Utilities|Struct|BreakS_PlayerInfo _array_element_3)) 0)
          (Variables|Default|SetCanWeStart? false)
          (CallFunction|CannotStartGame)
          (else
            (Variables|Default|SetCanWeStart? true)))))))

(event Custom|AddToKickList
  ;[1 1 1] Adds connected players to kick list
  (bind _lobbypc (Class|BPILobbyPC|LobbyPCRef(Message) (Game|GetPlayerController 0)))
  (Default|AddPlayertoKickWindow _lobbypc))

(event Custom|CannotStartGame
  ;[1 1 1] Updates All Connected players for lobby widget
  (Utilities|Array|ForEachLoopwithBreak (Variables|Default|GetConnectPlayersInfo)) ; enters at Break
)

(event Custom|LaunchGame
  (bind _returnvalue (Game|GetPlayerController 0))
  ;[1 1 1] Show loading screen and loads level
  (switch int (Variables|Default|GetSelectedMapID)
    (:0
      (Development|ExecuteConsoleCommand "servertravel /Game/Levels/TimeOfDayGameplayMap" _returnvalue))
    (:1
      (Development|ExecuteConsoleCommand "servertravel /Game/Levels/JungleWarfareGamePlayer" _returnvalue))))

(event Custom|ChangeCharcter
  (params (ConnectedPlayer :type Player%20Controller%20Object%20Reference) (CharacterClass :type Character%20Class%20Reference) (ChangedStatus :type Boolean))
  (bind _spawnpoints (Variables|Default|GetSpawnPoints))
  ;[1 1 1] Spans the character selected
  (if (not ChangedStatus)
    (Utilities|IsValid (Pawn|GetControlledPawn ConnectedPlayer)
      (:Is%20Valid
        (Actor|DestroyActor))
      (:Is%20Not%20Valid
        _))
    (bind _returnvalue (Game|SpawnActorfromClass CharacterClass (Transformation|GetActorTransform (Utilities|Array|Get(acopy) _spawnpoints (- (Utilities|Array|Length _spawnpoints) 1))) "AlwaysSpawn" 0 0))
    (Pawn|Possess ConnectedPlayer _returnvalue)))

(event EventOnLogout
  (params (ExitingController :type Controller%20Object%20Reference))
  (bind _connectedplayers (Variables|Default|GetConnectedPlayers))
  ;[1 1 1] Removes Connected Player infoa nd maeks veryone update whiloe reavailablizing the character
  (bind (_array_element _array_index) (Utilities|Array|ForEachLoopwithBreak _connectedplayers :!label _label)
    (:LoopBody
      (if (== _array_element ExitingController)
        (goto _label Break)))
    (:Completed
      (bind _lobbypc (Class|BPILobbyPC|LobbyPCRef(Message) (Utilities|Array|Get(acopy) _connectedplayers _array_index)))
      (Utilities|Array|SetArrayElem (Variables|Default|GetAvailableCharacters) (Variables|/Game/_Main/Lobby/BP_LobbyPC.BP_LobbyPC_C|GetSelectedCharacter _lobbypc) false)
      (Utilities|Array|RemoveIndex (Variables|Default|GetConnectedPlayers) _array_index)
      (Utilities|Array|RemoveIndex (Variables|Default|GetConnectPlayersInfo) _array_index)
      (CallFunction|EveryoneUpdate))))

(event EventPostLogin
  (params (NewPlayer :type Player%20Controller%20Object%20Reference))
  ;[1 1 1] Initial setup that runs eachtime player joins the agme
  (bind _output_get (Variables|Default|SetConnectedPlayer NewPlayer))
  (Utilities|Array|AddUnique (Variables|Default|GetConnectedPlayers) _output_get)
  (bind _outactors (Actor|GetAllActorsOfClass "/Script/Engine.PlayerStart"))
  (Variables|Default|SetSpawnPoints _outactors)
  (bind _gameinstance (Class|BPIGameInstance|SteamGameInstanceRef(Message) (Game|GetGameInstance)))
  (Variables|Default|SetServername (Variables|/Game/_Main/SteamGameInstance.SteamGameInstance_C|GetServer%20Name _gameinstance))
  (Variables|Default|SetMaxPlayers (Variables|/Game/_Main/SteamGameInstance.SteamGameInstance_C|GetMaxPlayers _gameinstance))
  (bind _lobbypc (Class|BPILobbyPC|LobbyPCRef(Message) (Variables|Default|GetConnectedPlayer)))
  (bind _output_get_2 (Variables|Default|SetLobbyPC _lobbypc))
  (Default|InitialSetup _output_get_2)
  (Default|SetupLobbyMenu (Variables|Default|GetLobbyPC) (Variables|Default|GetServername))
  (Default|UpdateLobbySettings (Variables|Default|GetLobbyPC) (Variables|Default|GetSelectedMapImagre) (Variables|Default|GetSelectedMapName) (Variables|Default|GetSelectedMapTime))
  (CallFunction|EveryoneUpdate))

(fn ConstructionScript)

(fn LobbyGMRef
  (return self))